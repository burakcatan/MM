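; Lobby game mode that creates the lobby menu widget on post-login and handles hosting or joining LAN multiplayer sessions.
; HostGame creates a session and opens DoorAndLeverLevel as a listen server, while JoinGame joins the first session found.
; Both pass the player name to the game instance on success for later use, and report failures through the lobby widget.
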(event EventBeginPlay)

(event EventTick
  (params (DeltaSeconds :type Float%20%28single-precision%29)))

(event EventJoinGame
  (params (Name :type Text%20%28by%20ref%29))
  ;[1 1 1] Join Game
  ;;[1 1 1] Find available sessions and join the first one (can be extended as selection from a list)
  (bind _results (|FindSessions (Game|GetPlayerController 0) 5 true)
    (:OnSuccess
      (if (> (Utilities|Array|Length _results) 0)
        (|JoinSession (Game|GetPlayerController 0) (Utilities|Array|Get(acopy) _results)
          (:OnSuccess
            ;;[1 1 1] Store player name in game instance for later
            (Class|MMPlayerDetailsInterface|SetPlayerName(Message) (Game|GetGameInstance) Name))
          (:OnFailure
            (Default|ShowErrorMessage (Variables|Default|GetLobbyMenuWidget) "Failed to while joining the session")))
        (else
          (Default|ShowErrorMessage (Variables|Default|GetLobbyMenuWidget) "Failed to find sessions"))))
    (:OnFailure
      (Default|ShowErrorMessage (Variables|Default|GetLobbyMenuWidget) "Failed to find sessions"))))

(event EventPostLogin
  (params (NewPlayer :type Player%20Controller%20Object%20Reference))
  ;[1 1 1] OnPostLogin: Create lobby widget
  (bind _returnvalue (UserInterface|CreateWidget "/Game/Task/Widgets/WBP_LobbyMenu.WBP_LobbyMenu_C" NewPlayer))
  (bind _output_get (Variables|Default|SetLobbyMenuWidget _returnvalue))
  (UserInterface|Viewport|AddtoViewport _output_get 0))

(event EventHostGame
  (params (Name :type Text%20%28by%20ref%29))
  ;[1 1 1] Host Game
  ;;[1 1 1] Create a session
  (|Session (Game|GetPlayerController 0) 5 true
    (:OnSuccess
      ;;[1 1 1] Open the level with ?listen option
      (Game|OpenLevel(byObjectReference) "/Game/Task/Maps/DoorAndLeverLevel.DoorAndLeverLevel" true "?listen")
      ;;[1 1 1] Store player name in game instance for later
      (Class|MMPlayerDetailsInterface|SetPlayerName(Message) (Game|GetGameInstance) Name))
    (:OnFailure
      (Default|ShowErrorMessage (Variables|Default|GetLobbyMenuWidget) "Failed to create session"))))

(fn ConstructionScript)