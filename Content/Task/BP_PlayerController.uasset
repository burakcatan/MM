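; Player controller that passes the player's lobby-entered name to their character and handles interaction input.
; On BeginPlay it copies the name from the game instance to pawn 0, then creates the interaction info widget and sets game-only input for local controllers only.
; The Interact input sends an interface message to every overlapping actor implementing MMInteractionInterface, through an event intended to run on the server.
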(event Custom|Interact
  (params (Target :type Object%20Object%20Reference))
  ;[1 1 1] Input Interact
  ;;[1 1 1] Interaction should be handled by server
  (Class|MMInteractionInterface|Interact(Message) Target))

(event EventBeginPlay
  ;[1 1 1] BeginPlay: Get player name from the game instance (we stored in the lobby GM), pass it to the player character
  (bind _returnvalue (Class|MMPlayerDetailsInterface|GetPlayerName(Message) (Game|GetGameInstance)))
  (Class|MMPlayerDetailsInterface|SetPlayerName(Message) (Game|Player|GetPlayerPawn 0) _returnvalue)
  ;[1 1 1] Create widget for interaction info
  ;;[1 1 1] Check if PC is local, otherwise it will try to add it on server instances as well
  (if (Pawn|IsLocalPlayerController)
    (bind _returnvalue_2 (UserInterface|CreateWidget "/Game/Task/Widgets/WBP_Info.WBP_Info_C" self))
    (UserInterface|Viewport|AddtoViewport _returnvalue_2 0)
    (Input|SetInputModeGameOnly self)))

(event Input|ActionEvents|InputActionInteract
  (params (Key :type Key%20Structure :default "None"))
  ;[1 1 1] Input Interact
  (:Pressed
    ;;[1 1 1] Get overlapping actors
    (for _array_element (Collision|GetOverlappingActors (Game|Player|GetPlayerPawn 0) 0 :!class /Script/Engine.Actor)
      ;;[1 1 1] If they have interaction interface, interact with them
      (if (Utilities|DoesObjectImplementInterface _array_element "/Script/MM.MMInteractionInterface")
        (CallFunction|Interact _array_element)))))

(fn ConstructionScript)